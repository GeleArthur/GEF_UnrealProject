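; BP_EnemyCharacter is an enemy character that deals repeated damage to a player overlapping it.
; On overlap with a BP_PlayerCharacter it stores the target and starts a looping timer, which sends damage to the player's BPCHealth component at the attack interval.
; End overlap with that target requests clearing the timer by function name.
; The Construction Script creates a dynamic material on the mesh to apply the enemy's body color.
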(event Custom|Damage%20Player
  (bind _currentplayertarget (Variables|Default|GetCurrentPlayerTarget))
  (Utilities|IsValid _currentplayertarget
    (:Is%20Valid
      (Class|BPIDamage|Damage(Message) (Variables|/Game/Blueprints/BP_Base_Character.BP_Base_Character_C|GetBPC_Health _currentplayertarget) (Variables|Default|GetDamageAmount)))))

(event EventBeginPlay
  (|CallParentFunction) ; This node is disabled and will not be called.\nDrag off pins to build functionality.
)

(event Collision|EventActorBeginOverlap
  (params (OtherActor :type Actor%20Object%20Reference))
  (|CallParentFunction OtherActor)
  (bind _asbp_player_character (Utilities|Casting|CastToBP_PlayerCharacter OtherActor))
  (Variables|Default|SetCurrentPlayerTarget _asbp_player_character)
  (Utilities|Time|SetTimerbyEvent (delegate Custom|Damage%20Player) (Variables|Default|GetAttackInterval) true))

(event EventTick
  (params (DeltaSeconds :type Float%20%28single-precision%29))
  (|CallParentFunction DeltaSeconds) ; This node is disabled and will not be called.\nDrag off pins to build functionality.
)

(event Collision|EventActorEndOverlap
  (params (OtherActor :type Actor%20Object%20Reference))
  (if (== OtherActor (Variables|Default|GetCurrentPlayerTarget))
    (Utilities|Time|ClearTimerbyFunctionName 0 "Damage Player")))

(fn ConstructionScript
  (|CallParentFunction)
  (bind _returnvalue (Rendering|Material|CreateDynamicMaterialInstance (Variables|Character|GetMesh) 0 0 "None" :!class /Script/Engine.PrimitiveComponent))
  (bind _output_get (Variables|Default|SetBodyMatriall _returnvalue))
  (Rendering|Material|SetVectorParameterValue _output_get "BodyColor" (Variables|Enemey|GetEnemyColor) :!class /Script/Engine.MaterialInstanceDynamic))