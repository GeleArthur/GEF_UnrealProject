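; BP_PlayerCharacter is the player character that carries a weapon and handles its own death.
; On BeginPlay it spawns the StartWeapon class, falling back to BP_BaseWeapon if unset, and snaps it to GunSocket as CurrentWeapon.
; Primary and secondary fire events forward their start/stop flag to that weapon when valid.
; BPC_Health's OnDeath event destroys both the weapon and the character.
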(event OnDeath(BPC_Health)
  (Actor|DestroyActor (Variables|Weapon|GetCurrentWeapon)))

(event Custom|Primary%20Fire
  (params (IsStart :type Boolean))
  (bind _currentweapon (Variables|Weapon|GetCurrentWeapon)
    (:then
      (Default|FirePrimary _currentweapon IsStart))
    (:else)))

(event Custom|Secondary%20Fire
  (params (IsStart :type Boolean))
  (bind _currentweapon (Variables|Weapon|GetCurrentWeapon)
    (:then
      (Default|FireSecondary _currentweapon IsStart))
    (:else)))

(event EventBeginPlay
  (bind _gunsocket (Variables|Default|GetGunSocket))
  (bind _startweapon (Variables|Weapon|GetStartWeapon))
  (|CallParentFunction)
  (bind _asbp_base_weapon (Utilities|Casting|CastToBP_BaseWeaponClass (Class|KismetMathLibrary|SelectClass _startweapon "/Game/Blueprints/BP_BaseWeapon.BP_BaseWeapon_C" (Utilities|IsValidClass _startweapon))))
  ;[1 1 1] Spawn and attched gun
  (bind _returnvalue (Game|SpawnActorfromClass _asbp_base_weapon (Transformation|GetWorldTransform _gunsocket) "Undefined" "MultiplyWithRoot" 0 0))
  (bind _output_get (Variables|Weapon|SetCurrentWeapon _returnvalue))
  (Transformation|AttachComponentToComponent _output_get _gunsocket "None" "SnapToTarget" "SnapToTarget" "SnapToTarget" true))

(event Collision|EventActorBeginOverlap
  (params (OtherActor :type Actor%20Object%20Reference))
  (|CallParentFunction OtherActor) ; This node is disabled and will not be called.\nDrag off pins to build functionality.
)

(event EventTick
  (params (DeltaSeconds :type Float%20%28single-precision%29))
  (|CallParentFunction DeltaSeconds) ; This node is disabled and will not be called.\nDrag off pins to build functionality.
)

(fn ConstructionScript
  (|CallParentFunction))