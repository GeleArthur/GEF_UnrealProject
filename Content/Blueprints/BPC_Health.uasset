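; BPC_Health is a health component that tracks current health against a maximum and signals death.
; It resets to full health on BeginPlay or through the ResetHealth event.
; Damage subtracts a clamped amount, fires OnDeath only when that hit lowers health to zero, and returns whether the owner is dead.
; Death is derived from the health percentage rather than a stored flag.
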(event Custom|Reset%20Health
  (Variables|Default|SetCurrentHeatlh (Variables|Default|GetMaxHealth)))

(event EventBeginPlay
  (CallFunction|ResetHealth))

(event EventTick
  (params (DeltaSeconds :type Float%20%28single-precision%29)))

(fn GetHealthPercentage
  (return (/ (Variables|Default|GetCurrentHeatlh) (Variables|Default|GetMaxHealth))))

(fn IsDead
  (return (<= (CallFunction|GetHealthPercentage) 0.0)))

(fn Damage
  (params (Amount :type Float%20%28double-precision%29))
  (bind _isdead (CallFunction|IsDead))
  (LocalVariables|SetLastHealth (Variables|Default|GetCurrentHeatlh))
  (bind _output_get (Variables|Default|SetCurrentHeatlh (Math|Float|Clamp(Float) (- (Variables|Default|GetCurrentHeatlh) Amount) 0.0 (Variables|Default|GetMaxHealth))))
  (if (and _isdead (> (LocalVariables|GetLastHealth) _output_get))
    (Default|CallOnDeath))
  (return _isdead))