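; Game mode that starts continuous enemy spawning and handles player respawn.
; On BeginPlay it gathers every BP_EnemySpawner in the level and sets a looping timer on each to call its Spawn function at an interval derived from EnemiesPerSecond.
; PlayerRespawn spawns the default pawn at a player start and has player controller 0 possess it.
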(event Custom|PlayerRespawn
  (bind _returnvalue (Game|GetPlayerController 0))
  (bind _returnvalue_2 (Game|SpawnActorfromClass (Variables|Default|GetDefaultPawnClass) (Transformation|GetActorTransform (Class|GameModeBase|FindPlayerStart _returnvalue)) "Undefined" "MultiplyWithRoot" 0 0))
  (Pawn|Possess _returnvalue _returnvalue_2))

(event EventBeginPlay
  (bind _outactors (Actor|GetAllActorsOfClass "/Game/Blueprints/BP_EnemySpawner.BP_EnemySpawner_C"))
  (bind _output_get (Variables|Default|SetEnemySpawners _outactors))
  (for _array_element _output_get
    (Utilities|Time|SetTimerbyFunctionName _array_element "Spawn" (/ 1.0 (Variables|Default|GetEnemiesPerSecond)) true)))

(fn ConstructionScript)