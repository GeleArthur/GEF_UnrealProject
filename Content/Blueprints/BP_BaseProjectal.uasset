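; Base projectile actor that damages whatever its sphere hits or overlaps, skipping anything tagged Friendly.
; Both sphere events feed ProcessCollision, which sends DamageAmount through the BPI_Damage interface to the other actor, then destroys the projectile.
; Damage also goes to the target's first BPI_Damage components via a short index loop that breaks if the target becomes invalid.
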(event OnComponentHit(Sphere)
  (params (HitComponent :type Primitive%20Component%20Object%20Reference) (OtherActor :type Actor%20Object%20Reference) (OtherComp :type Primitive%20Component%20Object%20Reference) (NormalImpulse :type Vector :default "0, 0, 0") (Hit :type Hit%20Result%20Structure%20%28by%20ref%29))
  (CallFunction|ProcessCollision OtherActor))

(event OnComponentBeginOverlap(Sphere)
  (params (OverlappedComponent :type Primitive%20Component%20Object%20Reference) (OtherActor :type Actor%20Object%20Reference) (OtherComp :type Primitive%20Component%20Object%20Reference) (OtherBodyIndex :type Integer) (bFromSweep :type Boolean) (SweepResult :type Hit%20Result%20Structure%20%28by%20ref%29))
  (CallFunction|ProcessCollision OtherActor))

(event EventBeginPlay)

(event Collision|EventActorBeginOverlap
  (params (OtherActor :type Actor%20Object%20Reference)))

(event EventTick
  (params (DeltaSeconds :type Float%20%28single-precision%29)))

(fn ConstructionScript)

(fn ProcessCollision
  (params (HitCollider :type Actor%20Object%20Reference))
  (bind _returnvalue (Class|Actor|GetComponentsbyInterface HitCollider "/Game/Blueprints/BPI_Damage.BPI_Damage_C"))
  (Utilities|IsValid HitCollider
    (:Is%20Valid
      ;[1 1 1] Friendly Check
      (if (not (Actor|ActorHasTag HitCollider "Friendly"))
        (Utilities|FlowControl|Sequence
          (:then_0
            (if (Utilities|DoesObjectImplementInterface HitCollider "/Game/Blueprints/BPI_Damage.BPI_Damage_C")
              (Class|BPIDamage|Damage(Message) HitCollider (Variables|Default|GetDamageAmount))))
          (:then_1
            ;[1 1 1] Do funny for loop so we can check if the object is delete before we go and try again
            (Utilities|IsValid HitCollider
              (:Is%20Valid
                (bind _index (Utilities|FlowControl|ForLoopwithBreak 0 (Math|Integer|Min(Integer) (Utilities|Array|Length _returnvalue) 1) :!label _label)
                  (:LoopBody
                    (Class|BPIDamage|Damage(Message) (Utilities|Array|Get(acopy) _returnvalue _index) (Variables|Default|GetDamageAmount))
                    (Utilities|IsValid HitCollider
                      (:Is%20Not%20Valid
                        (goto _label Break))))))))
          (:then_2
            (Actor|DestroyActor)))))))