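; BP_PlayerPawn is the player-controlled pawn, moving on the horizontal plane and turning to face its direction of travel.
; On BeginPlay it adds the IMC_default Enhanced Input mapping context to the player's subsystem.
; IA_PlayerMovement applies a swept world-space offset from clamped input, scaled by Speed and delta time, and stores the heading as DesiredRotation.
; Tick lerps the actor's rotation toward that target along the shortest path.
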(event Input|EnhancedActionEvents|EnhancedInputActionIA_PlayerMovement
  (params (ActionValue :type Vector%202D%20Structure) (ElapsedSeconds :type Float%20%28double-precision%29) (TriggeredSeconds :type Float%20%28double-precision%29) (InputAction :type Input%20Action%20Object%20Reference :default "/Game/Input/Actions/IA_PlayerMovement.IA_PlayerMovement"))
  (bind _returnvalue (Utilities|Time|GetWorldDeltaSeconds))
  (bind _returnvalue_2 (Math|Vector|MakeVector (.y ActionValue) (.x ActionValue) 0.0))
  (bind _speed (Variables|PawnMovment|GetSpeed))
  (bind _returnvalue_3 (Math|Vector|ClampVectorSize _returnvalue_2 0.0 1.0))
  (bind _returnvalue_4 (* _returnvalue _returnvalue_3))
  (bind _returnvalue_5 (* _returnvalue_4 _speed))
  (:Triggered
    (Transformation|AddActorWorldOffset _returnvalue_5 true)
    (if (> (Math|Vector|VectorLength _returnvalue_5) 0.0)
      (Variables|Default|SetDesiredRotation (Math|Conversions|RotationFromXVector _returnvalue_5)))))

(event EventBeginPlay
  ;[1 1 1] Comment
  (bind _asplayer_controller (Utilities|Casting|CastToPlayerController (Pawn|GetController)))
  (Utilities|IsValid (PlayerController|LocalPlayerSubsystems|GetEnhancedInputLocalPlayerSubsystem _asplayer_controller)
    (:Is%20Valid
      (Input|AddMappingContext (PlayerController|LocalPlayerSubsystems|GetEnhancedInputLocalPlayerSubsystem _asplayer_controller) "/Game/Input/IMC_default.IMC_default" 0 "(bIgnoreAllPressedKeysUntilRelease=True,bForceImmediately=False)"))))

(event Collision|EventActorBeginOverlap
  (params (OtherActor :type Actor%20Object%20Reference)))

(event EventTick
  (params (DeltaSeconds :type Float%20%28single-precision%29))
  (Transformation|SetActorRotation (Math|Rotator|Lerp(Rotator) (Transformation|GetActorRotation) (Variables|Default|GetDesiredRotation) (* (Variables|Default|GetRotationSpeed) DeltaSeconds) true)))

(fn ConstructionScript)